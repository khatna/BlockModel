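; BP_BlockModel colors the groups of a block model built on Runtime Mesh Components.
; Its PostprocessBlocks event walks the keys of the BlockGroups map and creates a dynamic instance of BlockMaterial_Inst for each group.
; Each instance takes its BaseColor from the Colors array by key index, wrapping around with modulo, and is assigned to that group's first material slot.
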(event EventPostprocessBlocks
  (bind _keys (Utilities|Map|Keys (Variables|Default|GetBlockGroups)))
  (for (_array_element _array_index) _keys
    (bind _returnvalue (Rendering|Material|CreateDynamicMaterialInstance (Variables|/Script/RuntimeMeshComponent.RuntimeMeshActor|GetRuntimeMeshComponent (.Value (Utilities|Map|Find (Variables|Default|GetBlockGroups) _array_element))) 0 "/BlockModel/Materials/BlockMaterial_Inst.BlockMaterial_Inst" "None" :!class /Script/Engine.PrimitiveComponent))
    (Rendering|Material|SetVectorParameterValue _returnvalue "BaseColor" (Math|Conversions|ToLinearColor(Color) (Utilities|Array|Get(acopy) (Variables|Default|GetColors) (Math|Integer|%(Integer) _array_index (Utilities|Array|Length (Variables|Default|GetColors))))) :!class /Script/Engine.MaterialInstanceDynamic)
    (Class|RuntimeMeshComponent|SetupMaterialSlot (Variables|/Script/RuntimeMeshComponent.RuntimeMeshActor|GetRuntimeMeshComponent (.Value (Utilities|Map|Find (Variables|Default|GetBlockGroups) _array_element))) 0 "None" _returnvalue)))